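; Left-hand VR motion controller that shows a holographic oxygen readout, extending a parent controller's logic.
; Every tick it formats O2Value from MotionControllerPawn_RB into the InfoTextO2 text.
; The text and hologram cone appear only while a BP_MotionController_Right_LB actor overlaps the ShowInfoO2 trigger.
; The InfoO2 swatch widget is mirrored and linked at BeginPlay, but its animated show/hide chains are disconnected.
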(event OnComponentBeginOverlap(ShowInfoO2)
  (params (OverlappedComponent :type Primitive%20Component%20Object%20Reference) (OtherActor :type Actor%20Object%20Reference) (OtherComp :type Primitive%20Component%20Object%20Reference) (OtherBodyIndex :type Integer) (bFromSweep :type Boolean) (SweepResult :type Hit%20Result%20Structure%20%28by%20ref%29))
  (Utilities|Casting|CastToBP_MotionController_Right_LB OtherActor)
  (Rendering|SetVisibility (Variables|Default|GetInfoTextO2) true false)
  (Rendering|SetVisibility (Variables|Default|GetConeHolo) true false))

(event OnComponentEndOverlap(ShowInfoO2)
  (params (OverlappedComponent :type Primitive%20Component%20Object%20Reference) (OtherActor :type Actor%20Object%20Reference) (OtherComp :type Primitive%20Component%20Object%20Reference) (OtherBodyIndex :type Integer))
  (Utilities|Casting|CastToBP_MotionController_Right_LB OtherActor)
  (Rendering|SetVisibility (Variables|Default|GetInfoTextO2) false false)
  (Rendering|SetVisibility (Variables|Default|GetConeHolo) false false))

(event EventBeginPlay
  (bind _infoo2 (Variables|Default|GetInfoO2))
  (bind _returnvalue (UserInterface|GetUserWidgetObject _infoo2))
  (bind _aswg_info_swatch (Utilities|Casting|CastToWG_InfoSwatch _returnvalue))
  (|CallParentFunction)
  (Transformation|SetRelativeScale3D _infoo2 "1.000000,1.000000,-1.000000")
  (Variables|Default|SetWidgetHolo _aswg_info_swatch)
  (Variables|/Game/Widgets/WG_InfoSwatch.WG_InfoSwatch_C|SetBP_MotionLeft _aswg_info_swatch self)
  (Class|TextRenderComponent|SetTextMaterial (Variables|Default|GetInfoTextO2) "/Game/Blueprints/Character/Romain/DefaultTextMaterialOpaque_RB_2.DefaultTextMaterialOpaque_RB_2"))

(event Collision|EventActorBeginOverlap
  (params (OtherActor :type Actor%20Object%20Reference)))

(event EventTick
  (params (DeltaSeconds :type Float%20%28single-precision%29))
  (|CallParentFunction DeltaSeconds)
  (bind _output_get (Variables|Default|SetO2_Text (Utilities|Text|ToText(String) (Utilities|String|Append "O2 : " (Utilities|String|ToString(Text) (Utilities|Text|ToText(Float) (Variables|/Game/Blueprints/Character/MotionControllerPawn_RB.MotionControllerPawn_RB_C|GetO2Value (.AsMotion%20Controller%20Pawn%20RB (Utilities|Casting|CastToMotionControllerPawn_RB (Game|Player|GetPlayerPawn 0)))) "HalfToEven" false true 1 2 0 2))))))
  (Rendering|Components|TextRender|SetText (Variables|Default|GetInfoTextO2) _output_get))

(fn ConstructionScript
  (|CallParentFunction))