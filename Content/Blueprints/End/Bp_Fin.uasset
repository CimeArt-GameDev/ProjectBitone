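; Bp_Fin is an end-goal zone that counts BPP_ObjInterract objects inside its sphere toward a target of six.
; Overlap events add or remove objects from an array, and each entry restarts the Niagara effect.
; Below six, and on every exit, it prints the missing count and recolors the circle and Niagara by array length.
; Reaching six on entry only prints "fini" after the effect, with no further completion logic.
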(event OnComponentBeginOverlap(Sphere)
  (params (OverlappedComponent :type Primitive%20Component%20Object%20Reference) (OtherActor :type Actor%20Object%20Reference) (OtherComp :type Primitive%20Component%20Object%20Reference) (OtherBodyIndex :type Integer) (bFromSweep :type Boolean) (SweepResult :type Hit%20Result%20Structure%20%28by%20ref%29))
  (bind _actor (Variables|Default|Getactor))
  (bind _actor_2 (Variables|Default|Getactor))
  (bind _returnvalue (Utilities|Array|Length _actor))
  (bind _returnvalue_2 (Utilities|Array|Length _actor_2))
  (bind _returnvalue_3 (Utilities|Select :Index _returnvalue_2 :Option%200 "(R=1.000000,G=1.000000,B=1.000000,A=1.000000)" :Option%201 "(R=1.000000,G=0.022553,B=0.000000,A=1.000000)" :Option%202 "(R=1.000000,G=0.000000,B=0.266000,A=1.000000)" :Option%203 "(R=1.000000,G=0.654823,B=0.000000,A=1.000000)" :Option%204 "(R=0.000000,G=0.963542,B=0.930098,A=1.000000)" :Option%205 "(R=0.000000,G=0.505208,B=0.020808,A=1.000000)"))
  (bind _asbpp_obj_interract (Utilities|Casting|CastToBPP_ObjInterract OtherActor))
  (Utilities|Array|Add _actor _asbpp_obj_interract)
  (CallFunction|VFX)
  (if (== _returnvalue 6)
    (Development|PrintString "fini")
    (else
      (Development|PrintString (Utilities|String|Append "il en manque " (Utilities|String|ToString(Integer) (- 6 _returnvalue))))
      (Effects|Components|ParticleSystem|SetColorParameter (Variables|Default|GetCircle) "Color" _returnvalue_3)
      (Effects|Components|ParticleSystem|SetColorParameter (Variables|Default|GetNiagara) "Color" _returnvalue_3))))

(event OnComponentEndOverlap(Sphere)
  (params (OverlappedComponent :type Primitive%20Component%20Object%20Reference) (OtherActor :type Actor%20Object%20Reference) (OtherComp :type Primitive%20Component%20Object%20Reference) (OtherBodyIndex :type Integer))
  (bind _actor (Variables|Default|Getactor))
  (bind _actor_2 (Variables|Default|Getactor))
  (bind _returnvalue (Utilities|Array|Length _actor_2))
  (bind _returnvalue_2 (Utilities|Select :Index _returnvalue :Option%200 "(R=1.000000,G=1.000000,B=1.000000,A=1.000000)" :Option%201 "(R=1.000000,G=0.022553,B=0.000000,A=1.000000)" :Option%202 "(R=1.000000,G=0.000000,B=0.266000,A=1.000000)" :Option%203 "(R=1.000000,G=0.654823,B=0.000000,A=1.000000)" :Option%204 "(R=0.000000,G=0.963542,B=0.930098,A=1.000000)" :Option%205 "(R=0.000000,G=0.505208,B=0.020808,A=1.000000)"))
  (bind _asbpp_obj_interract (Utilities|Casting|CastToBPP_ObjInterract OtherActor))
  (Utilities|Array|RemoveItem _actor _asbpp_obj_interract)
  (Development|PrintString (Utilities|String|Append "il en manque " (Utilities|String|ToString(Integer) (- 6 (Utilities|Array|Length _actor)))))
  (Effects|Components|ParticleSystem|SetColorParameter (Variables|Default|GetCircle) "Color" _returnvalue_2)
  (Effects|Components|ParticleSystem|SetColorParameter (Variables|Default|GetNiagara) "Color" _returnvalue_2))

(event Custom|VFX
  (bind _niagara (Variables|Default|GetNiagara))
  (Components|Activation|Activate _niagara false)
  (Niagara|ResetSystem _niagara))

(event EventBeginPlay)

(event Collision|EventActorBeginOverlap
  (params (OtherActor :type Actor%20Object%20Reference)))

(event EventTick
  (params (DeltaSeconds :type Float%20%28single-precision%29)))

(fn ConstructionScript)