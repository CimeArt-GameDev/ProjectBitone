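; BP_GrappleHook is a grappling hook projectile that pulls the player toward the point it hits.
; On BeginPlay its cable end attaches to the GrappleStart component on Hand.
; When the Hook component overlaps, it starts the player's grapple movement, passing its location and the direction toward it, and posts a Wwise whoosh event.
; It then destroys its projectile and rotating movement components, stopping the hook in place.
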(event OnComponentBeginOverlap(Hook)
  (params (OverlappedComponent :type Primitive%20Component%20Object%20Reference) (OtherActor :type Actor%20Object%20Reference) (OtherComp :type Primitive%20Component%20Object%20Reference) (OtherBodyIndex :type Integer) (bFromSweep :type Boolean) (SweepResult :type Hit%20Result%20Structure%20%28by%20ref%29))
  (bind _returnvalue (Transformation|GetActorLocation))
  (bind _projectilemovement (Variables|Default|GetProjectileMovement))
  (bind _player (Variables|Default|GetPlayer))
  (Default|StartGrapplemovement _player (Math|Vector|GetForwardVector (Math|Rotator|FindLookatRotation (Transformation|GetActorLocation _player) _returnvalue)) _returnvalue)
  (Class|AkGameplayStatics|PostEvent "/Game/WwiseAudio/Events/Rudhy_WorkUnit/GrappleHook/Movement/Play_Whoosh_Sequence.Play_Whoosh_Sequence")
  (Utilities|IsValid _projectilemovement
    (:Is%20Valid
      (Components|DestroyComponent _projectilemovement))))

(event EventBeginPlay
  (Class|CableComponent|SetAttachEndtoComponent (Variables|Default|GetCable) (Variables|/Game/VirtualRealityBP/Blueprints/BP_MotionController.BP_MotionController_C|GetGrappleStart (Variables|Default|GetHand)) "None"))

(event Collision|EventActorBeginOverlap
  (params (OtherActor :type Actor%20Object%20Reference)))

(event EventTick
  (params (DeltaSeconds :type Float%20%28single-precision%29)))

(fn ConstructionScript)