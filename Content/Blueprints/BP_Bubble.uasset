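; BP_Bubble is an oxygen bubble that raises or lowers the player's O2 on the MotionControllerPawn_RB pawn.
; Overlap events on its Cone set an Inside flag, without checking which actor overlaps.
; Every Tick, it calls IncreaseO2 on player pawn 0 while its Niagara effect is active and Inside is true, otherwise DecreaseO2, so each placed instance drains oxygen whenever those conditions fail.
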(event OnComponentBeginOverlap(Cone)
  (params (OverlappedComponent :type Primitive%20Component%20Object%20Reference) (OtherActor :type Actor%20Object%20Reference) (OtherComp :type Primitive%20Component%20Object%20Reference) (OtherBodyIndex :type Integer) (bFromSweep :type Boolean) (SweepResult :type Hit%20Result%20Structure%20%28by%20ref%29))
  (Variables|Default|Setinside? true))

(event OnComponentEndOverlap(Cone)
  (params (OverlappedComponent :type Primitive%20Component%20Object%20Reference) (OtherActor :type Actor%20Object%20Reference) (OtherComp :type Primitive%20Component%20Object%20Reference) (OtherBodyIndex :type Integer))
  (Variables|Default|Setinside? false))

(event EventBeginPlay)

(event Collision|EventActorBeginOverlap
  (params (OtherActor :type Actor%20Object%20Reference)))

(event EventTick
  (params (DeltaSeconds :type Float%20%28single-precision%29))
  (if (and (Components|Activation|IsActive (Variables|Default|GetNiagara)) (Variables|Default|Getinside?))
    (bind _asmotion_controller_pawn_rb (Utilities|Casting|CastToMotionControllerPawn_RB (Game|Player|GetPlayerPawn 0)))
    (Default|IncreaseO2 _asmotion_controller_pawn_rb)
    (else
      (bind _asmotion_controller_pawn_rb_2 (Utilities|Casting|CastToMotionControllerPawn_RB (Game|Player|GetPlayerPawn 0)))
      (Default|DecreaseO2 _asmotion_controller_pawn_rb_2))))

(fn ConstructionScript)