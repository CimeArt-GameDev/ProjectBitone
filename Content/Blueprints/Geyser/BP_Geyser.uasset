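; BP_Geyser is a geyser actor that erupts on a repeating cycle through a Niagara effect.
; From BeginPlay, Timeline_0 event tracks activate and deactivate the effect, and the timeline restarts after a fixed delay each time it finishes.
; Unconnected leftovers hold a cast to HMDLocomotionPawn and a timeline-driven pushback, but the overlap events are empty, so the geyser affects nothing it touches.
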(event OnComponentBeginOverlap(Niagara)
  (params (OverlappedComponent :type Primitive%20Component%20Object%20Reference) (OtherActor :type Actor%20Object%20Reference) (OtherComp :type Primitive%20Component%20Object%20Reference) (OtherBodyIndex :type Integer) (bFromSweep :type Boolean) (SweepResult :type Hit%20Result%20Structure%20%28by%20ref%29)))

(event EventBeginPlay
  (bind _niagara (Variables|Default|GetNiagara))
  (Timeline|Timeline_0 PlayFromStart
    (:Finished
      (Utilities|FlowControl|Delay 5.0)
      (Timeline|Timeline_0 PlayFromStart))
    (:NewTrack_2
      (Components|Activation|Activate _niagara true))
    (:NewTrack_3
      (Components|Activation|Deactivate _niagara))))

(event Collision|EventActorBeginOverlap
  (params (OtherActor :type Actor%20Object%20Reference)))

(event EventTick
  (params (DeltaSeconds :type Float%20%28single-precision%29)))

(fn ConstructionScript)