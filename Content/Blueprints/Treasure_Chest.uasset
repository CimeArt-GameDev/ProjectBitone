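; Treasure chest actor with a child BP_Bubble, flagging a MotionControllerPawn_RB as in a bubble while it overlaps the chest's box.
; An Opening timeline is set up to swing the lid open and shut after a delay, toggling the bubble's Niagara effect via event tracks.
; Nothing in the graph starts that timeline, and the bubble-active check is disconnected, so overlap sets the flag unconditionally.
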(event OnComponentBeginOverlap(Box)
  (params (OverlappedComponent :type Primitive%20Component%20Object%20Reference) (OtherActor :type Actor%20Object%20Reference) (OtherComp :type Primitive%20Component%20Object%20Reference) (OtherBodyIndex :type Integer) (bFromSweep :type Boolean) (SweepResult :type Hit%20Result%20Structure%20%28by%20ref%29))
  ;[1 1 1] A REVOIR
  (bind _asmotion_controller_pawn_rb (Utilities|Casting|CastToMotionControllerPawn_RB OtherActor))
  (Variables|/Game/Blueprints/Character/MotionControllerPawn_RB.MotionControllerPawn_RB_C|SetIsInBubulle _asmotion_controller_pawn_rb true))

(event OnComponentEndOverlap(Box)
  (params (OverlappedComponent :type Primitive%20Component%20Object%20Reference) (OtherActor :type Actor%20Object%20Reference) (OtherComp :type Primitive%20Component%20Object%20Reference) (OtherBodyIndex :type Integer))
  ;[1 1 1] A REVOIR
  (bind _asmotion_controller_pawn_rb (Utilities|Casting|CastToMotionControllerPawn_RB OtherActor))
  (Variables|/Game/Blueprints/Character/MotionControllerPawn_RB.MotionControllerPawn_RB_C|SetIsInBubulle _asmotion_controller_pawn_rb false))

(event EventBeginPlay
  (Variables|Default|SetBP_Bubble (.AsBP%20Bubble (Utilities|Casting|CastToBP_Bubble (Variables|/Script/Engine.ChildActorComponent|GetChildActor (Variables|Default|GetChildActor))))))

(fn ConstructionScript)